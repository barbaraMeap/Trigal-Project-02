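; BP_InspectItem is an inspectable world item actor that shows a configurable mesh and can be picked up.
; The construction script applies the ItemModel variable to its static mesh component.
; NewFunction prints a pickup debug message, triggers DestroItem and returns ItemModel to the caller.
; DestroItem destroys the actor after a short delay.
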(event `DestroItem`
  (`KismetSystemLibrary.Delay` 0.2)
  (`self.K2_DestroyActor`))

(fn `NewFunction`
  (returns (ItemModel :type "StaticMesh Object Reference"))
  (`KismetSystemLibrary.PrintString` "Item agarrdo")
  (`self.DestroItem`)
  (return (`self.ItemModel`)))

(fn `UserConstructionScript`
  (`StaticMeshComponent.SetStaticMesh` (`self.StaticMesh`) (`self.ItemModel`)))